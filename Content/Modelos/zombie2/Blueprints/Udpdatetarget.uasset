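; Behavior tree service for the zombie AI that updates its target based on how close the player is.
; Each tick it compares squared distance between the controlled pawn and player character 0 against the squared perception distance.
; Within range, it writes the player to the target blackboard key and switches the AI state enum; otherwise it clears the target and sets the other state.
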(event `self.ReceiveTickAI`
  (params (OwnerController :type "AIController Object Reference") (ControlledPawn :type "Pawn Object Reference") (DeltaSeconds :type "Float (single-precision)"))
  (if (< (`KismetMathLibrary.Vector_DistanceSquared` (`Actor.K2_GetActorLocation` ControlledPawn) (`Actor.K2_GetActorLocation` (`GameplayStatics.GetPlayerCharacter` 0))) (`KismetMathLibrary.Square` (`self.Perceptiondistance`)))
    (`BTFunctionLibrary.SetBlackboardValueAsObject` (`self.AiTarget`) (`GameplayStatics.GetPlayerCharacter` 0))
    (`BTFunctionLibrary.SetBlackboardValueAsEnum` (`self.AiState`) (enumliteral `/Game/Modelos/zombie2/Blueprints/ZombieAIstate` "NewEnumerator1"))
    (else
      (`BTFunctionLibrary.SetBlackboardValueAsObject` (`self.AiTarget`))
      (`BTFunctionLibrary.SetBlackboardValueAsEnum` (`self.AiState`) (enumliteral `/Game/Modelos/zombie2/Blueprints/ZombieAIstate` "NewEnumerator0")))))