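; Zombie enemy character that damages actors it overlaps and turns into a ragdoll when killed.
; On BeginPlay it randomizes mesh scale per axis and walk speed for variety between instances, and sets its rotation.
; Overlaps send a fixed damage message to the other actor.
; Kill stops the AI brain logic, switches the mesh to physics and changes capsule collision, then after a delay fires OnKilled and destroys the actor.
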(event `self.ReceiveBeginPlay`
  (bind _returnvalue (`KismetMathLibrary.RandomFloatInRange` 0.9 1.1))
  (`|ExecutionSequence`
    (:`then_0`
      (`SceneComponent.SetWorldScale3D` (`self.Mesh`) (`KismetMathLibrary.MakeVector` _returnvalue _returnvalue _returnvalue))
      (`self.K2_SetActorRotation` (`KismetMathLibrary.MakeRotator` 0.0))
      (set `CharacterMovementComponent.MaxWalkSpeed` (`KismetMathLibrary.RandomFloatInRange` 450.0 700.0) (`self.CharacterMovement`)))))

(event `self.ReceiveActorBeginOverlap`
  (params (OtherActor :type "Actor Object Reference"))
  (message `/Game/FirstPersonBP/Blueprints/BP_Damagle.Take Damage` OtherActor 20.0))

(event `Kill`
  (bind _mesh (`self.Mesh`))
  (`BrainComponent.StopLogic` (`AIController.BrainComponent` (`AIBlueprintHelperLibrary.GetAIController` self)) "")
  (`PrimitiveComponent.SetCollisionProfileName` _mesh "Ragdoll" true)
  (`PrimitiveComponent.SetSimulatePhysics` _mesh true)
  (`PrimitiveComponent.SetCollisionProfileName` (`self.CapsuleComponent`) "NoColision" true)
  (`KismetSystemLibrary.Delay` 2.0)
  (`self.OnKilled` self)
  (`self.K2_DestroyActor`))

(fn `UserConstructionScript`)